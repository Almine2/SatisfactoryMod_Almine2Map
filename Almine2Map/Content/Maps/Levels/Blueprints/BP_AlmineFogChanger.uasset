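; Level actor for Almine2Map that switches between inside and outside height fog and plays the map's music.
; Player height picks the initial fog after a delay, then InBox and OutBox overlaps swap visibility, guarded by IsOut.
; Tick plays the first track below the height threshold or a random other above it, with config-driven volume and randomized gaps between tracks.
; Fog tag lookup and BP_MusicManager hookup are unconnected leftovers.
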(event `self.ReceiveBeginPlay`
  (`KismetSystemLibrary.Delay` 5.0)
  (if (< (`.Z` (`KismetMathLibrary.BreakVector3f` (`self.K2_GetActorLocation` (`GameplayStatics.GetPlayerPawn` 0)))) -17620.0)
    (set `self.IsOut` false)
    (`SceneComponent.SetVisibility` (`ExponentialHeightFog.Component` (`self.Fog1`)) true false)
    (`SceneComponent.SetVisibility` (`ExponentialHeightFog.Component` (`self.Fog2`)) false false)
    (else
      (set `self.IsOut` true)
      (`SceneComponent.SetVisibility` (`ExponentialHeightFog.Component` (`self.Fog1`)) false false)
      (`SceneComponent.SetVisibility` (`ExponentialHeightFog.Component` (`self.Fog2`)) true false))))

(event `self.ReceiveTick`
  (params (DeltaSeconds :type "Float (single-precision)"))
  (bind _audio (`self.Audio`))
  (bind _musiclists (`self.MusicLists`))
  (if (not (`AudioComponent.IsPlaying` _audio))
    (bind _output_get (set `self.Counter` (+ (`self.Counter`) DeltaSeconds)))
    (if (> _output_get (`self.NextMusicTime`))
      (set `self.Counter` 0.0)
      (if (< (`.Z` (`KismetMathLibrary.BreakVector3f` (`self.K2_GetActorLocation` (`GameplayStatics.GetPlayerPawn` 0)))) -17620.0)
        (`AudioComponent.SetSound` _audio (`|GetArrayItem` _musiclists))
        (else
          (`AudioComponent.SetSound` _audio (`|GetArrayItem` _musiclists (`KismetMathLibrary.RandomIntegerInRange` 1 (- (`KismetArrayLibrary.Array_Length` _musiclists) 1))))))
      (bind _asbp_config_property_section (cast `/SML/Interface/UI/Menu/Mods/ConfigProperties/BP_ConfigPropertySection` (`RuntimeBlueprintFunctionLibrary.Conv_ModConfigurationToConfigProperty` "/Almine2Map/Almine2Map_Config.Almine2Map_Config_C"))
        (:`then`
          (`AudioComponent.SetVolumeMultiplier` _audio (`RuntimeBlueprintFunctionLibrary.Conv_ConfigPropertyToFloat` (`RuntimeBlueprintFunctionLibrary.Conv_ConfigPropertySectionToConfigProperty` _asbp_config_property_section "MusicVolume"))))
        (:`CastFailed`
          (`AudioComponent.SetVolumeMultiplier` _audio 0.5)))
      (`AudioComponent.Play` _audio 0.0))))

(event `self.Audio.OnAudioFinished`
  (set `self.NextMusicTime` (`KismetMathLibrary.RandomFloatInRange` 20.0 300.0)))

(event `self.InBox.OnComponentBeginOverlap`
  (params (OverlappedComponent :type "PrimitiveComponent Object Reference") (OtherActor :type "Actor Object Reference") (OtherComp :type "PrimitiveComponent Object Reference") (OtherBodyIndex :type Integer) (bFromSweep :type Boolean) (SweepResult :type "HitResult Structure (by ref)"))
  (if (`self.IsOut`)
    (`SceneComponent.SetVisibility` (`ExponentialHeightFog.Component` (`self.Fog1`)) true false)
    (`SceneComponent.SetVisibility` (`ExponentialHeightFog.Component` (`self.Fog2`)) false false)
    (set `self.IsOut` false)))

(event `self.OutBox.OnComponentBeginOverlap`
  (params (OverlappedComponent :type "PrimitiveComponent Object Reference") (OtherActor :type "Actor Object Reference") (OtherComp :type "PrimitiveComponent Object Reference") (OtherBodyIndex :type Integer) (bFromSweep :type Boolean) (SweepResult :type "HitResult Structure (by ref)"))
  (if (not (`self.IsOut`))
    (`SceneComponent.SetVisibility` (`ExponentialHeightFog.Component` (`self.Fog2`)) true false)
    (`SceneComponent.SetVisibility` (`ExponentialHeightFog.Component` (`self.Fog1`)) false false)
    (set `self.IsOut` true)))

(fn `UserConstructionScript`)