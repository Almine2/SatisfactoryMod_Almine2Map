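; Sky actor for the Almine map that replaces the stock FGSkySphere and drives lighting from the game's time of day.
; BeginPlay adopts the level's height fog and tagged Sun and Moon lights, disables other directional lights, destroys sky spheres and applies a dynamic star material.
; Tick samples curves for light rotation and intensity, fog colour and night star alpha, while updating SkyLight intensity and overriding both atmosphere light directions.
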(event `self.ReceiveBeginPlay`
  (`BlueprintLoggingLibrary.LogVerbose` "Almine2Map : NogSky begin play")
  (`FGTimeOfDaySubsystem.SetTimeSpeedMultiplier` (`FGTimeOfDaySubsystem.Get` null) 1.0)
  (bind _returnvalue (`KismetMaterialLibrary.CreateDynamicMaterialInstance` (`self.MI_AlSky`) "MIAlSkyDynamic" "Transient"))
  (set `self.MI_AlSkyDynamic` _returnvalue)
  (`PrimitiveComponent.SetMaterial` (`self.SM_SkySphere_ExtraUV`) 0 _returnvalue)
  (`MaterialInstanceDynamic.SetScalarParameterValue` (`self.MI_AlSkyDynamic`) "Alpha" 0.0)
  (bind _outactors (`GameplayStatics.GetAllActorsOfClass` "/Script/Engine.ExponentialHeightFog"))
  (set `self.Fog` (`|GetArrayItem` _outactors))
  (bind _outactors_2 (`GameplayStatics.GetAllActorsOfClass` "/Script/Engine.DirectionalLight"))
  (for _array_element _outactors_2
    (if (`self.ActorHasTag` _array_element "Sun")
      (set `self.Sun` _array_element)
      (elif (`self.ActorHasTag` _array_element "Moon")
        (set `self.Moon` _array_element)
        (else
          (bind _lightcomponent (`Light.LightComponent` _array_element))
          (`LightComponent.SetIntensity` _lightcomponent 0.0)
          (`SceneComponent.SetVisibility` _lightcomponent false false)
          (`self.SetActorHiddenInGame` _array_element true)))))
  (bind _outactors_3 (`GameplayStatics.GetAllActorsOfClass` "/Script/FactoryGame.FGSkySphere"))
  (for _array_element_2 _outactors_3
    (`self.K2_DestroyActor` _array_element_2)))

(event `self.ReceiveTick`
  (params (DeltaSeconds :type "Float (single-precision)"))
  (bind _returnvalue (`FGTimeOfDaySubsystem.Get` null))
  (bind _returnvalue_2 (`FGTimeOfDaySubsystem.Get` null))
  (bind _fog (`self.Fog`))
  (bind _sun (`self.Sun`))
  (bind _moon (`self.Moon`))
  (bind _skyatomosphere (`self.SkyAtomosphere`))
  (bind _skylight (`self.SkyLight`))
  (bind _returnvalue_3 (`FGTimeOfDaySubsystem.GetNormalizedTimeOfDay` _returnvalue_2))
  (bind (_x _y _z) (`KismetMathLibrary.BreakVector3f` (`CurveVector.GetVectorValue` (`self.MoonRotationCurve`) _returnvalue_3)))
  (bind (_x_2 _y_2 _z_2) (`KismetMathLibrary.BreakVector3f` (`CurveVector.GetVectorValue` (`self.SunRotationCurve`) _returnvalue_3)))
  (`/Engine/EditorBlueprintResources/StandardMacros.IsValid` _returnvalue
    (:`Is Valid`
      (`|ExecutionSequence`
        (:`then_0`
          (`SceneComponent.K2_SetRelativeRotation` (`Actor.RootComponent` _sun) (`KismetMathLibrary.MakeRotator` _x_2 _y_2 _z_2) false true)
          (`LightComponent.SetIntensity` (`Light.LightComponent` _sun) (`KismetMathLibrary.BreakVector3f` (`CurveVector.GetVectorValue` (`self.IntensityCurve`) _returnvalue_3)))
          (`/Engine/EditorBlueprintResources/StandardMacros.IsValid` _skylight
            (:`Is Valid`
              (`SkyLightComponent.SetIntensity` _skylight (`KismetMathLibrary.FClamp` (`FGTimeOfDaySubsystem.GetDayPct` _returnvalue) 0.3 0.9))
              (`/Engine/EditorBlueprintResources/StandardMacros.IsValid` _skyatomosphere
                (:`Is Valid`
                  (`SkyAtmosphereComponent.OverrideAtmosphereLightDirection` (`SkyAtmosphere.SkyAtmosphereComponent` _skyatomosphere) 0 (* (`SceneComponent.GetForwardVector` (`Actor.RootComponent` _sun)) (-1.0 -1.0 -1.0))))))
            (:`Is Not Valid`
              (`BlueprintLoggingLibrary.LogError` "SkyLight Invalid"))))
        (:`then_1`
          (`SceneComponent.K2_SetRelativeRotation` (`Actor.RootComponent` _moon) (`KismetMathLibrary.MakeRotator` _x _y _z) false true)
          (`LightComponent.SetIntensity` (`Light.LightComponent` _moon) (`.Y` (`KismetMathLibrary.BreakVector3f` (`CurveVector.GetVectorValue` (`self.IntensityCurve`) _returnvalue_3))))
          (`MaterialInstanceDynamic.SetScalarParameterValue` (`self.MI_AlSkyDynamic`) "Alpha" (`CurveFloat.GetFloatValue` (`self.StarCurve`) (* (- (`FGTimeOfDaySubsystem.GetNightPct` _returnvalue) 0.495) 2.0)))
          (`SkyAtmosphereComponent.OverrideAtmosphereLightDirection` (`SkyAtmosphere.SkyAtmosphereComponent` _skyatomosphere) 1 (* (`SceneComponent.GetForwardVector` (`Actor.RootComponent` _moon)) -1.0)))
        (:`then_2`
          (`/Engine/EditorBlueprintResources/StandardMacros.IsValid` _fog
            (:`Is Valid`
              (`ExponentialHeightFogComponent.SetFogInscatteringColor` (`ExponentialHeightFog.Component` _fog) (`CurveLinearColor.GetLinearColorValue` (`self.Curve`) (/ (`FGTimeOfDaySubsystem.GetTimeOfDayHours` _returnvalue_2) 24.0))))))))))

(fn `UserConstructionScript`)